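; Player spaceship actor that turns, thrusts and fires projectiles, driven by rotation, thruster and shooter variables that are set outside these graphs.
; Each Tick applies yaw while zeroing pitch and roll, then sets capsule physics velocity forward or to zero, without inertia.
; Firing spawns BP_Projectile at the mesh's FireSocket, limited by a time-since-last-shot check.
; The projectile velocity node is unconnected, and ReduceHealth is an empty stub.
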(event EventBeginPlay
  (Variables|Buttons|SetThrusterIsPressed false)
  (Variables|Buttons|SetShooterIsPressed false))

(event EventTick
  (params (DeltaSeconds :type Float%20%28single-precision%29))
  (Movement|RotateSpaceship)
  (Movement|MoveSpaceship)
  (Firing|SpawnProjectile))

(fn ConstructionScript)

(fn RotateSpaceship
  (Transformation|AddActorLocalRotation (Math|Rotator|MakeRotator 0.0 0.0 (* (Variables|Movement|GetRotationValue) 0.5)) false false)
  (Transformation|SetActorRotation (Math|Rotator|MakeRotator 0.0 0.0 (.yaw (Transformation|GetActorRotation)))))

(fn MoveSpaceship
  (if (Variables|Buttons|GetThrusterIsPressed)
    (Physics|SetPhysicsLinearVelocity (Variables|Default|GetCapsuleComponent) (* (Transformation|GetActorForwardVector) 1e+02) false "None")
    (else
      (Physics|SetPhysicsLinearVelocity (Variables|Default|GetCapsuleComponent) "0, 0, 0" false "None"))))

(fn SpawnProjectile
  (if (Variables|Buttons|GetShooterIsPressed)
    (bind _canshoot (Firing|CheckifCanShoot))
    (if _canshoot
      (Variables|Firing|SetTimeOfLastFire (Actor|GetGameTimeSinceCreation))
      (bind _returnvalue (Game|SpawnActorfromClass "/Game/BP_Projectile.BP_Projectile_C" (Transformation|GetSocketTransform (Variables|Default|GetSpaceshipMesh) "FireSocket" "RTS_World") "Undefined" 0 0)))))

(fn CheckifCanShoot
  (return (> (- (Actor|GetGameTimeSinceCreation) (Variables|Firing|GetTimeOfLastFire)) (Variables|Firing|GetRateOfFire))))

(fn ReduceHealth)