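; BP_Star is a star actor that pulls every BP_SpaceShip toward itself with simulated gravity.
; Each Tick it finds all ships and applies CalculateGravity's result to their meshes as a velocity-change impulse, unscaled by delta time.
; The pull multiplies both masses and two gravity constants over squared distance, times the unnormalized offset vector, so it falls off with distance rather than its square.
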(event EventBeginPlay)

(event Collision|EventActorBeginOverlap
  (params (OtherActor :type Actor%20Object%20Reference)))

(event EventTick
  (params (DeltaSeconds :type Float%20%28single-precision%29))
  (bind _outactors (Actor|GetAllActorsOfClass "/Game/BP_SpaceShip.BP_SpaceShip_C"))
  (for _array_element _outactors
    (bind _starforce (CallFunction|CalculateGravity _array_element))
    (Physics|AddImpulse (Variables|/Game/BP_SpaceShip.BP_SpaceShip_C|GetSpaceshipMesh _array_element) _starforce "None" true)))

(fn ConstructionScript)

(fn CalculateGravity
  (params (Spaceship :type BP%20Space%20Ship%20Object%20Reference))
  (return (* (- (Transformation|GetActorLocation) (Transformation|GetActorLocation Spaceship)) (* (* (/ (* (Physics|GetMass (Variables|/Game/BP_SpaceShip.BP_SpaceShip_C|GetSpaceshipMesh Spaceship)) (Physics|GetMass (Variables|Default|GetSphere))) (Transformation|GetSquaredDistanceTo Spaceship)) (Variables|Default|GetGravityConstant_0)) (Variables|Default|GetGravityConstant_1)))))