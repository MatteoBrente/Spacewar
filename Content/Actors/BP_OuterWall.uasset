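; BP_OuterWall is a boundary wall that wraps any overlapping actor around to the opposite side of the play area.
; On begin overlap, IsHorizontalWall selects the axis: horizontal walls change X through TeleportVertically, others change Y through TeleportHorizontally.
; Each function negates that coordinate and adds TeleportDistance, keeps the other two, and moves the actor with the teleport flag set.
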(event Collision|EventActorBeginOverlap
  (params (OtherActor :type Actor%20Object%20Reference))
  (if (Variables|Default|GetIsHorizontalWall)
    (CallFunction|TeleportVertically OtherActor)
    (else
      (CallFunction|TeleportHorizontally OtherActor))))

(fn ConstructionScript)

(fn TeleportHorizontally
  (params (OtherActor :type Actor%20Object%20Reference))
  (bind _returnvalue (Transformation|GetActorLocation OtherActor))
  (Transformation|SetActorLocation OtherActor (Math|Vector|MakeVector (.x _returnvalue) (+ (* (.y _returnvalue) -1.0) (Variables|Default|GetTeleportDistance)) (.z _returnvalue)) false true))

(fn TeleportVertically
  (params (OtherActor :type Actor%20Object%20Reference))
  (bind _returnvalue (Transformation|GetActorLocation OtherActor))
  (Transformation|SetActorLocation OtherActor (Math|Vector|MakeVector (+ (* (.x _returnvalue) -1.0) (Variables|Default|GetTeleportDistance)) (.y _returnvalue) (.z _returnvalue)) false true))