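; BP_Star is a star actor that exerts gravitational pull on every BP_SpaceShip in the level.
; Each Tick it gathers all ships with GetAllActorsOfClass and applies a force to each SpaceshipMesh toward the star.
; CalculateGravity multiplies both meshes' masses by GravityConstant over squared distance, then scales the unnormalized offset vector, so pull falls off with distance rather than its square.
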(event EventTick
  (params (DeltaSeconds :type Float%20%28single-precision%29))
  (bind _outactors (Actor|GetAllActorsOfClass "/Game/Actors/BP_SpaceShip.BP_SpaceShip_C"))
  (for _array_element _outactors
    (bind _starforce (CallFunction|CalculateGravity _array_element))
    (Physics|AddForce (Variables|/Game/Actors/BP_SpaceShip.BP_SpaceShip_C|GetSpaceshipMesh _array_element) _starforce "None" false)))

(fn ConstructionScript)

(fn CalculateGravity
  (params (Spaceship :type BP%20Space%20Ship%20Object%20Reference))
  (return (* (- (Transformation|GetActorLocation) (Transformation|GetActorLocation Spaceship)) (* (/ (* (Physics|GetMass (Variables|/Game/Actors/BP_SpaceShip.BP_SpaceShip_C|GetSpaceshipMesh Spaceship)) (Physics|GetMass (Variables|Default|GetSphere))) (Transformation|GetSquaredDistanceTo Spaceship)) (Variables|Default|GetGravityConstant)))))